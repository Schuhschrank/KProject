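; Bullet impact effect actor that leaves a hit decal and plays an impact sound where it spawns.
; On BeginPlay it spawns the decal at its own transform, tied to the actor's initial lifespan, with a tiny fade screen size to keep it visible at distance.
; Only the authority triggers the multicast event that plays the sound cue at the impact location.
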(event `self.ReceiveBeginPlay`
  (bind _returnvalue (`GameplayStatics.SpawnDecalAtLocation` "/Game/Materials/M_Decal_Hit.M_Decal_Hit" (4.0 8.0 8.0) (`self.K2_GetActorLocation`) (`self.K2_GetActorRotation`) (`self.InitialLifeSpan`)))
  (`DecalComponent.SetFadeScreenSize` _returnvalue 0.001)
  (`/Engine/EditorBlueprintResources/ActorMacros.Switch Has Authority`
    (:`Authority`
      (`self.Multicast_PlaySound`))))

(event `Multicast_PlaySound`
  (`GameplayStatics.PlaySoundAtLocation` "/Game/Audio/bullet_impact_Cue.bullet_impact_Cue" (`self.K2_GetActorLocation`) (struct) 1.0 1.0 0.0 null null self))

(fn `UserConstructionScript`)
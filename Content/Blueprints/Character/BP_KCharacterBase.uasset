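; Base character Blueprint that sets up positional voice chat for the character.
; On BeginPlay it adds a VOIPTalker, polls with a capped delay loop until PlayerState is valid, then registers it and applies mic threshold, mesh attachment, attenuation and effect chain.
; Failures print on-screen errors, and EndPlay deactivates and destroys the talker.
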(event `self.ReceiveBeginPlay`
  ;[1 1 1] Set up positional voice chat
  (bind _returnvalue (`AddComponent|NODE_AddVOIPTalker-0`))
  (bind _output_get (set `self.VOIP` _returnvalue))
  (`/Engine/EditorBlueprintResources/StandardMacros.IsValid` _output_get
    (:`Is Valid`
      (bind _counter (`/Engine/EditorBlueprintResources/StandardMacros.Do N` 100 :!label _label)
        (:`Exit`
          (if (< _counter 99)
            (`/Engine/EditorBlueprintResources/StandardMacros.IsValid` (`self.PlayerState`)
              (:`Is Valid`
                (`VOIPTalker.RegisterWithPlayerState` (`self.VOIP`) (`self.PlayerState`))
                (`VOIPStatics.SetMicThreshold` -1.0)
                (set `VOIPTalker.Settings` (make `VoiceSettings` (`self.Mesh`) "/Game/Blueprints/Character/VOIPAttenuation.VOIPAttenuation" "/Game/Blueprints/Character/VOIPSoundEffectSourcePresetChain.VOIPSoundEffectSourcePresetChain") (`self.VOIP`)))
              (:`Is Not Valid`
                (`KismetSystemLibrary.Delay` 0.2)
                (goto _label)))
            (else
              (`KismetSystemLibrary.PrintString` "Error: VOIP Could not get PlayerState" true true (struct :`R` 1.0 :`A` 1.0) 10.0))))))
    (:`Is Not Valid`
      (`KismetSystemLibrary.PrintString` "Error: Could not add VOIPTalker" true true (struct :`R` 1.0 :`A` 1.0) 10.0))))

(event `self.ReceiveEndPlay`
  (params (EndPlayReason :type "EEndPlayReason Enum" :default "Destroyed"))
  (bind _voip (`self.VOIP`))
  ;[1 1 1] Clean up positional voice chat
  (`ActorComponent.Deactivate` _voip)
  (`ActorComponent.K2_DestroyComponent` _voip))

(fn `UserConstructionScript`)
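; Networked player character for a shooter, with hitscan pistol fire, interaction and death handling.
; Use input, throttled by DoOnce and a delay, has the server trace from the eyes, apply damage and spawn impacts, then multicast sound and weapon animation.
; Interact sends a short server trace that messages the hit actor; death notifies BP_KGameMode, and health prints on screen locally.
; The separate Gun actor's spawn and Use logic is disconnected.
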(event `Multicast_BulletFired`
  (`GameplayStatics.PlaySoundAtLocation` "/Game/Audio/fart_noise_Cue.fart_noise_Cue" (`self.K2_GetActorLocation`) (struct) 1.0 1.0 0.0 null null self)
  (`SkeletalMeshComponent.PlayAnimation` (`self.Weapon`) "/Game/Blueprints/Items/PrototypePistol/PrototypePistol_Anim.PrototypePistol_Anim" false))

(event `Server_Use`
  (bind (_outlocation _outrotation) (`self.GetActorEyesViewPoint`))
  (`|ExecutionSequence`
    (:`then_0`
      (bind _outhit (`KismetSystemLibrary.LineTraceSingle` _outlocation (+ _outlocation (* (`KismetMathLibrary.GetForwardVector` _outrotation) 20000.0)) "TraceTypeQuery3"))
      (bind (_bblockinghit _binitialoverlap _time _distance _location _impactpoint _normal _impactnormal _physmat _hitactor) (`GameplayStatics.BreakHitResult` _outhit))
      (if _bblockinghit
        (`GameplayStatics.ApplyDamage` _hitactor 25.0 (`self.GetController`) self)
        (`|SpawnActorFromClass` "/Game/Blueprints/BP_BulletImpact.BP_BulletImpact_C" (`KismetMathLibrary.MakeTransform` _location (`KismetMathLibrary.Conv_VectorToRotator` _normal)) "Undefined" "OverrideRootScale" null null)))
    (:`then_1`
      (`self.Multicast_BulletFired`))))

(event `InputAction|Use`
  (params (Key :type "Key Structure"))
  (:`Pressed`
    (`/Engine/EditorBlueprintResources/StandardMacros.DoOnce` false :!label _label
      (:`Completed`
        (`self.Server_Use`)
        (`KismetSystemLibrary.Delay` 0.2)
        (goto _label :!via `Reset`)))))

(event `Server_StopUsing`
  (bind _gun (`self.Gun`))
  (`/Engine/EditorBlueprintResources/StandardMacros.IsValid` _gun
    (:`Is Valid`
      (`/Game/Blueprints/Items/BP_AK47.StopUsing` _gun))))

(event `InputAction|Interact`
  (params (Key :type "Key Structure"))
  (:`Pressed`
    (`self.Server_Interact`)))

(event `Server_Interact`
  (bind (_outlocation _outrotation) (`self.GetActorEyesViewPoint`))
  (bind _outhit (`KismetSystemLibrary.LineTraceSingle` :`Start` _outlocation :`End` (+ _outlocation (* (`KismetMathLibrary.GetForwardVector` _outrotation) 200.0)) :`TraceChannel` "TraceTypeQuery1" :`DrawDebugType` "ForDuration"))
  (bind (_bblockinghit _binitialoverlap _time _distance _location _impactpoint _normal _impactnormal _physmat _hitactor) (`GameplayStatics.BreakHitResult` _outhit))
  (if _bblockinghit
    (message `/Game/Blueprints/BI_Generic.Interact` _hitactor)))

(event `self.HealthComponent.OnDeath`
  (`KismetSystemLibrary.PrintString` "I died!")
  (bind _asbp_kgame_mode (cast `/Game/Blueprints/GameFramework/BP_KGameMode` (`GameplayStatics.GetGameMode`)))
  (`KGameMode.HandlePlayerDeath` _asbp_kgame_mode (`self.GetController`)))

(event `self.ReceiveEndPlay`
  (params (EndPlayReason :type "EEndPlayReason Enum" :default "Destroyed"))
  (bind _gun (`self.Gun`))
  (`/Engine/EditorBlueprintResources/ActorMacros.Switch Has Authority`
    (:`Authority`
      (`/Engine/EditorBlueprintResources/StandardMacros.IsValid` _gun
        (:`Is Valid`
          (`self.K2_DestroyActor` _gun))))))

(fn `ReceiveBeginPlay`)

(fn `ReceiveTick`
  (params (DeltaSeconds :type "Float (double-precision)"))
  (if (`self.IsLocallyControlled`)
    (`KismetSystemLibrary.PrintText` (`|FormatText` "Health: {hp}" (`/Game/Blueprints/HealthComponent.GetCurrentHealth` (`self.HealthComponent`))) true false (struct :`G` 0.66 :`B` 1.0 :`A` 1.0) 0.0)))

(fn `UserConstructionScript`
  (`parent.UserConstructionScript`))
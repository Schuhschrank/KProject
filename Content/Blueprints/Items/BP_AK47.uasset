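; AK-47 item Blueprint that acts as an automatic hitscan weapon for the character using it.
; Use runs only on the server, storing the user, firing immediately, then starting a looping timer for repeat shots until StopUsing clears it.
; FireBullet line-traces from the user's eye viewpoint, with debug drawing enabled, and applies flat damage to the blocking hit, crediting the user's controller.
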(fn `FireBullet`
  (bind _user (`self.User`))
  (bind (_outlocation _outrotation) (`self.GetActorEyesViewPoint` _user))
  (`/Engine/EditorBlueprintResources/StandardMacros.IsValid` _user
    (:`Is Valid`
      (bind _outhit (`KismetSystemLibrary.LineTraceSingle` _outlocation (+ _outlocation (* (`KismetMathLibrary.GetForwardVector` _outrotation) 20000.0)) "TraceTypeQuery3" false (`|MakeArray` (`self.User`) :!type "Actor Object Reference") "ForDuration"))
      (bind (_bblockinghit _binitialoverlap _time _distance _location _impactpoint _normal _impactnormal _physmat _hitactor) (`GameplayStatics.BreakHitResult` _outhit))
      (if _bblockinghit
        (`GameplayStatics.ApplyDamage` _hitactor 25.0 (`Pawn.GetController` (`self.User`)) self)))))

(fn `StopUsing`
  (`KismetSystemLibrary.K2_ClearAndInvalidateTimerHandle` (`self.FiringTimerHandle`)))

(fn `Use`
  (params (InUser :type "Pawn Object Reference"))
  (`/Engine/EditorBlueprintResources/ActorMacros.Switch Has Authority`
    (:`Authority`
      (bind _output_get (set `self.User` InUser))
      (`/Engine/EditorBlueprintResources/StandardMacros.IsValid` _output_get
        (:`Is Valid`
          (`self.FireBullet`)
          (bind _returnvalue (`KismetSystemLibrary.K2_SetTimerDelegate` (`|CreateDelegate` :!event `FireBullet`) 0.1 true))
          (set `self.FiringTimerHandle` _returnvalue))))))

(fn `UserConstructionScript`)
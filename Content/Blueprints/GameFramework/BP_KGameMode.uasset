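; BP_KGameMode is the game mode for a hidden-role match of traitors against innocents and detectives.
; It starts the match after a short delay, assigns roles, makes players mortal, and runs timers after the match ends or aborts.
; Deaths and logouts respawn players while immortal, otherwise make them spectating ghosts and check whether either side is wiped out.
; It records the end reason and multicasts logins and logouts through BP_KGameState.
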(event `self.ReceiveBeginPlay`
  (`KismetSystemLibrary.Delay` 2.0)
  (`self.StartMatch`))

(fn `HandlePlayerDeath`
  (params (DeadPlayer :type "Controller Object Reference"))
  (locals (PlayerState :type "/Game/Blueprints/GameFramework/BP_KPlayerState Object Reference"))
  (bind _playerstate (`Controller.PlayerState` (`local.DeadPlayer`)))
  (`/Engine/EditorBlueprintResources/StandardMacros.IsValid` DeadPlayer
    (:`Is Valid`
      (`|ExecutionSequence`
        (:`then_0`
          (`/Engine/EditorBlueprintResources/StandardMacros.IsValid` _playerstate
            (:`Is Valid`
              (bind _asbp_kplayer_state (cast `/Game/Blueprints/GameFramework/BP_KPlayerState` _playerstate))
              (bind _output_get (set `local.PlayerState` _asbp_kplayer_state))
              (if (or (`KPlayerState.IsGhost` _output_get) (`|EnumEquality` (`KPlayerState.GetPlayerRole` _output_get) "NotParticipating"))
                (return)))))
        (:`then_1`
          (if (not (`self.ArePlayersMortal`))
            (`self.RestartPlayer` (`local.DeadPlayer`))
            (return)
            (else
              (`|ExecutionSequence`
                (:`then_0`
                  (bind _playerstate_2 (`local.PlayerState`)
                    (:`then`
                      (`KPlayerState.SetIsGhost` _playerstate_2 true))
                    (:`else`)))
                (:`then_1`
                  (`self.MakePlayerSpectate` (`local.DeadPlayer`))
                  (bind _returnvalue (`self.ShouldEndMatch`))
                  (if _returnvalue
                    (`self.EndMatch`)
                    (return)))))))))
    (:`Is Not Valid`
      (return))))

(fn `K2_OnLogout`
  (params (ExitingController :type "Controller Object Reference"))
  (`/Engine/EditorBlueprintResources/StandardMacros.IsValid` ExitingController
    (:`Is Valid`
      (`self.HandlePlayerDeath` ExitingController)
      (bind _asbp_kgame_state (cast `/Game/Blueprints/GameFramework/BP_KGameState` (`GameplayStatics.GetGameState`)))
      (`/Game/Blueprints/GameFramework/BP_KGameState.Multicast_PlayerLoggedOut` _asbp_kgame_state (`Controller.PlayerState` (`local.ExitingController`))))))

(fn `K2_OnSetMatchState`
  (params (NewState :type Name))
  (switch `name` NewState
    (:`InProgress`
      (`self.DistributeRoles` 1)
      (`self.SetArePlayersMortal` true))
    (:`WaitingPostMatch`
      (`KismetSystemLibrary.K2_SetTimerDelegate` (`|CreateDelegate` :!event `RestartGame`) 5.0))
    (:`Aborted`
      (`KismetSystemLibrary.K2_SetTimerDelegate` (`|CreateDelegate` :!event `RestartGame`) 5.0))))

(fn `K2_PostLogin`
  (params (NewPlayer :type "PlayerController Object Reference"))
  (`/Engine/EditorBlueprintResources/StandardMacros.IsValid` NewPlayer
    (:`Is Valid`
      (bind _asbp_kgame_state (cast `/Game/Blueprints/GameFramework/BP_KGameState` (`GameplayStatics.GetGameState`)))
      (`/Game/Blueprints/GameFramework/BP_KGameState.Multicast_PlayerLoggedIn` _asbp_kgame_state (`AdvancedSessionsLibrary.GetPlayerName` NewPlayer)))))

(fn `KillAllPlayers`
  (for _array_element (`self.GetAllPlayers`)
    (`/Engine/EditorBlueprintResources/StandardMacros.IsValid` _array_element
      (:`Is Valid`
        (`self.HandlePlayerDeath` _array_element)))))

(fn `ShouldEndMatch`
  (returns (ReturnValue :type Boolean))
  (bind (_notparticipating _traitors _innocents _detectives) (break `RoleCounts` (`self.GetRoleCounts` true)))
  (if (`self.IsMatchInProgress`)
    (if (<= (+ _innocents _detectives) 0)
      (`|ExecutionSequence`
        (:`then_0`
          (bind _asbp_kgame_state (cast `/Game/Blueprints/GameFramework/BP_KGameState` (`GameplayStatics.GetGameState`)))
          (`/Game/Blueprints/GameFramework/BP_KGameState.SetEndMatchReason` _asbp_kgame_state "AllInnocentsDead"))
        (:`then_1`
          (return true)))
      (elif (<= _traitors 0)
        (`|ExecutionSequence`
          (:`then_0`
            (bind _asbp_kgame_state_2 (cast `/Game/Blueprints/GameFramework/BP_KGameState` (`GameplayStatics.GetGameState`)))
            (`/Game/Blueprints/GameFramework/BP_KGameState.SetEndMatchReason` _asbp_kgame_state_2 "AllTraitorsDead"))
          (:`then_1`
            (return true)))
        (else
          (return false))))
    (else
      (return false))))

(fn `ShouldReset`
  (params (ActorToReset :type "Actor Object Reference"))
  (returns (ReturnValue :type Boolean))
  (return (not (`.bSuccess` (cast `SpectatorPawn` ActorToReset :!pure true)))))

(fn `UserConstructionScript`)
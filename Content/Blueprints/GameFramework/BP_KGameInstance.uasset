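; BP_KGameInstance is the game instance, which owns the BP_SaveGame object for the session and reports network and travel errors.
; Init loads the save from its slot or creates a new one, a getter exposes it, and Shutdown writes it back.
; Error events only print red on-screen messages.
; Session destruction after errors and a frame-rate limit setup exist but are disconnected, so they never run.
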(event `self.HandleNetworkError`
  (params (FailureType :type "ENetworkFailure Enum" :default "NetDriverAlreadyExists") (bIsServer :type Boolean))
  (`KismetSystemLibrary.PrintText` (`|FormatText` "Network error: {type}, IsServer={server}" (`|GetEnumeratorNameAsString` FailureType) bIsServer) true true (struct :`R` 1.0 :`A` 1.0) 20.0))

(event `self.HandleTravelError`
  (params (FailureType :type "ETravelFailure Enum" :default "NoLevel"))
  (`KismetSystemLibrary.PrintText` (`|FormatText` "Travel error: {type}" (`|GetEnumeratorNameAsString` FailureType)) true true (struct :`R` 1.0 :`A` 1.0) 20.0))

(fn `GetSaveGame`
  (returns (`Save Game` :type "/Game/Blueprints/NonGameplay/BP_SaveGame Object Reference"))
  (return (`self.Save Game`)))

(fn `LoadSaveGame`
  (`|ExecutionSequence`
    (:`then_0`
      (bind _returnvalue (`GameplayStatics.DoesSaveGameExist` "default"))
      (if _returnvalue
        (bind _returnvalue_2 (`GameplayStatics.LoadGameFromSlot` (`self.SaveGameSlotName`)))
        (`/Engine/EditorBlueprintResources/StandardMacros.IsValid` _returnvalue_2
          (:`Is Valid`
            (bind _asbp_save_game (cast `/Game/Blueprints/NonGameplay/BP_SaveGame` _returnvalue_2))
            (set `self.Save Game` _asbp_save_game)))))
    (:`then_1`
      (`self.Save Game`
        (:`then`)
        (:`else`
          (bind _returnvalue_3 (`GameplayStatics.CreateSaveGameObject` "/Game/Blueprints/NonGameplay/BP_SaveGame.BP_SaveGame_C"))
          (set `self.Save Game` _returnvalue_3))))))

(fn `ReceiveInit`
  (`self.LoadSaveGame`))

(fn `ReceiveShutdown`
  (bind _save_game (`self.Save Game`)
    (:`then`
      (`GameplayStatics.SaveGameToSlot` _save_game (`self.SaveGameSlotName`)))
    (:`else`)))
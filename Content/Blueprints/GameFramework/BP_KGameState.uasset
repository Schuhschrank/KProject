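; BP_KGameState is a game state Blueprint that broadcasts match events through event dispatchers.
; Match state changes, player chat messages sent by multicast, and replicated end-match reason updates each fire their own dispatcher.
; The end-match reason has a setter and a RepNotify that announces changes.
; Tick prints the current match state on screen every frame as debug output.
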(event `self.OnMatchStateChanged`
  (`self.MatchStateChanged` (`self.MatchState`)))

(event `Multicast_SendMsg`
  (params (Sender :type "PlayerState Object Reference") (Msg :type String))
  (`self.PlayerSentMsg` Sender Msg))

(fn `OnRep_EndMatchReason`
  (`self.EndMatchReasonChanged` (`self.EndMatchReason`)))

(fn `ReceiveTick`
  (params (DeltaSeconds :type "Float (double-precision)"))
  (`KismetSystemLibrary.PrintString` (`KismetStringLibrary.Concat_StrStr` "Match state: " (`KismetStringLibrary.Conv_NameToString` (`self.MatchState`))) true false (struct :`G` 0.66 :`B` 1.0 :`A` 1.0) 0.0))

(fn `SetEndMatchReason`
  (params (NewEndMatchReason :type "EEndMatchReason Enum" :default "NoReason"))
  (set `self.EndMatchReason` NewEndMatchReason))

(fn `UserConstructionScript`)
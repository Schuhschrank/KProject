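; Player controller that owns the local UI: HUD with chat, in-game menu and a hold-P server info panel.
; On begin play the local controller creates these widgets, applies saved mouse sensitivity and binds their events, so chat toggles input mode and the menu disables chat while open.
; A server event relays chat through the game state's multicast.
; A test Die event calls the game mode, and Tick prints the player's role.
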(event `InputAction|OpenChat`
  (params (Key :type "Key Structure"))
  (:`Pressed`
    (`WidgetBlueprintLibrary.SetInputMode_UIOnlyEx` self (`/Game/UI/InGame/WB_Chat.Input` (`/Game/UI/InGame/WB_HUD.WB_Chat` (`self.HUD`))))))

(event `Server_SendMsg`
  (params (Msg :type String))
  (bind _playerstate (`self.PlayerState`))
  (bind _asbp_kgame_state (cast `/Game/Blueprints/GameFramework/BP_KGameState` (`GameplayStatics.GetGameState`)))
  (`/Engine/EditorBlueprintResources/StandardMacros.IsValid` _playerstate
    (:`Is Valid`
      (`/Game/Blueprints/GameFramework/BP_KGameState.Multicast_SendMsg` _asbp_kgame_state _playerstate Msg))))

(event `ChatClosed`
  (`KismetSystemLibrary.PrintString` "Chat closed")
  (`WidgetBlueprintLibrary.SetInputMode_GameOnly` self))

(event `InputAction|OpenMenu`
  (params (Key :type "Key Structure"))
  (bind _ingamemenu (`self.InGameMenu`))
  ;[1 1 1] Opening and closing in game menu
  (:`Pressed`
    (bind _ingamemenu_2 (`self.InGameMenu`)
      (:`then`
        (if (`/Game/UI/InGame/WB_InGameMenu.Is Open` _ingamemenu_2)
          (`/Game/UI/InGame/WB_InGameMenu.Close` _ingamemenu)
          (else
            (`/Game/UI/InGame/WB_InGameMenu.Open` _ingamemenu))))
      (:`else`))))

(event `Key|P`
  (params (Key :type "Key Structure"))
  (:`Pressed`
    (bind _serverinfo (`self.ServerInfo`)
      (:`then`
        (`UserWidget.AddToViewport` _serverinfo 0))
      (:`else`)))
  (:`Released`
    (bind _serverinfo_2 (`self.ServerInfo`)
      (:`then`
        (`Widget.RemoveFromParent` _serverinfo_2))
      (:`else`))))

(event `Die`
  (bind _asbp_kgame_mode (cast `/Game/Blueprints/GameFramework/BP_KGameMode` (`GameplayStatics.GetGameMode`)))
  (`KGameMode.HandlePlayerDeath` _asbp_kgame_mode self))

(event `InGameMenuOpened`
  (`/Game/UI/InGame/WB_Chat.Disable` (`/Game/UI/InGame/WB_HUD.WB_Chat` (`self.HUD`))))

(event `InGameMenuClosed`
  (`/Game/UI/InGame/WB_Chat.Enable` (`/Game/UI/InGame/WB_HUD.WB_Chat` (`self.HUD`))))

(fn `ReceiveBeginPlay`
  (if (`self.IsLocalPlayerController`)
    (`|ExecutionSequence`
      (:`then_0`
        (`WidgetBlueprintLibrary.SetInputMode_GameOnly` self)
        (set `self.bShowMouseCursor` false)
        (bind _asbp_kgame_instance (cast `/Game/Blueprints/GameFramework/BP_KGameInstance` (`GameplayStatics.GetGameInstance`)))
        (bind _save_game (`/Game/Blueprints/GameFramework/BP_KGameInstance.GetSaveGame` _asbp_kgame_instance))
        (`/Engine/EditorBlueprintResources/StandardMacros.IsValid` _save_game
          (:`Is Valid`
            (`self.SetMouseSensitivity` (`/Game/Blueprints/NonGameplay/BP_SaveGame.MouseSensitivity` _save_game)))))
      (:`then_1`
        (`|ExecutionSequence`
          (:`then_0`
            (bind _returnvalue (`|CreateWidget` "/Game/UI/InGame/WB_InGameMenu.WB_InGameMenu_C" self))
            (bind _output_get (set `self.InGameMenu` _returnvalue))
            (add `/Game/UI/InGame/WB_InGameMenu.Opened` _output_get (`|CreateDelegate` :!event `InGameMenuOpened`))
            (add `/Game/UI/InGame/WB_InGameMenu.Closed` _output_get (`|CreateDelegate` :!event `InGameMenuClosed`)))
          (:`then_1`
            (bind _returnvalue_2 (`|CreateWidget` "/Game/UI/InGame/WB_ServerInfo.WB_ServerInfo_C" self))
            (set `self.ServerInfo` _returnvalue_2))
          (:`then_2`
            (bind _returnvalue_3 (`|CreateWidget` "/Game/UI/InGame/WB_HUD.WB_HUD_C" self))
            (bind _output_get_2 (set `self.HUD` _returnvalue_3))
            (`UserWidget.AddToViewport` _output_get_2 0)
            (add `/Game/UI/InGame/WB_Chat.ChatClosed` (`/Game/UI/InGame/WB_HUD.WB_Chat` _output_get_2) (`|CreateDelegate` :!event `ChatClosed`))))))))

(fn `ReceiveTick`
  (params (DeltaSeconds :type "Float (double-precision)"))
  (bind _playerstate (`self.PlayerState`))
  (if (`self.IsLocalPlayerController`)
    (`/Engine/EditorBlueprintResources/StandardMacros.IsValid` _playerstate
      (:`Is Valid`
        (bind _asbp_kplayer_state (cast `/Game/Blueprints/GameFramework/BP_KPlayerState` _playerstate))
        (`KismetSystemLibrary.PrintString` (`KismetStringLibrary.Concat_StrStr` "Your role: " (`|GetEnumeratorNameAsString` (`KPlayerState.GetPlayerRole` _asbp_kplayer_state))) true false (struct :`G` 0.66 :`B` 1.0 :`A` 1.0) 0.0)))))

(fn `UserConstructionScript`)
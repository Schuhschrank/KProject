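; BP_KPlayerState is a player state Blueprint that handles replication and debug display of the player's role.
; On the authority, BeginPlay binds to the PlayerRoleChanged dispatcher, and each change forces a net update.
; Tick prints the current role on screen when the pawn is valid and locally controlled.
; The construction script and the bDummy rep notify are empty.
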(event `self.ReceiveBeginPlay`
  (`/Engine/EditorBlueprintResources/ActorMacros.Switch Has Authority`
    (:`Authority`
      (add `self.PlayerRoleChanged` (delegate `PlayerRoleChanged_Event_0`)))))

(event `PlayerRoleChanged_Event_0` :!signature `self.PlayerRoleChanged`
  (params (NewRole :type "EPlayerRole Enum" :default "NotParticipating"))
  (`/Engine/EditorBlueprintResources/ActorMacros.Switch Has Authority`
    (:`Authority`
      (`self.ForceNetUpdate`))))

(fn `OnRep_bDummy`)

(fn `ReceiveTick`
  (params (DeltaSeconds :type "Float (double-precision)"))
  (bind _pawnprivate (`self.PawnPrivate`))
  (`/Engine/EditorBlueprintResources/StandardMacros.IsValid` _pawnprivate
    (:`Is Valid`
      (if (`Pawn.IsLocallyControlled` _pawnprivate)
        (`KismetSystemLibrary.PrintString` (`|GetEnumeratorNameAsString` (`self.PlayerRole`)) true false (struct :`G` 0.66 :`B` 1.0 :`A` 1.0) 0.0)))))

(fn `UserConstructionScript`)
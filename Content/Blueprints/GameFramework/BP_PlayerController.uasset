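; Player controller that forwards match-flow requests to BP_GameMode through number-key bindings.
; Key 1 starts the match and key 3 restarts the game.
; Key 2 calls the Die event, which passes this controller to the game mode's HandlePlayerDeath.
; Each action casts the current game mode to BP_GameMode and does nothing if the cast fails.
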(event `Key|One`
  (params (Key :type "Key Structure"))
  (:`Pressed`
    (bind _asbp_game_mode (cast `/Game/Blueprints/GameFramework/BP_GameMode` (`GameplayStatics.GetGameMode`)))
    (`GameMode.StartMatch` _asbp_game_mode)))

(event `Die`
  (bind _asbp_game_mode (cast `/Game/Blueprints/GameFramework/BP_GameMode` (`GameplayStatics.GetGameMode`)))
  (`KGameMode.HandlePlayerDeath` _asbp_game_mode self))

(event `Key|Two`
  (params (Key :type "Key Structure"))
  (:`Pressed`
    (`self.Die`)))

(event `Key|Three`
  (params (Key :type "Key Structure"))
  (:`Pressed`
    (bind _asbp_game_mode (cast `/Game/Blueprints/GameFramework/BP_GameMode` (`GameplayStatics.GetGameMode`)))
    (`GameMode.RestartGame` _asbp_game_mode)))

(fn `UserConstructionScript`)
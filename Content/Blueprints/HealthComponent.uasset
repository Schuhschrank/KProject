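; Health component that tracks its owning actor's health and signals health changes and death.
; On the server or in standalone, it binds to the owner's any-damage event and subtracts damage, clamped at zero.
; At zero it makes the owner undamageable and fires OnDeath from that damage handler.
; CurrentHealth uses a RepNotify to broadcast OnHealthChanged, and getters expose health and alive state.
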(fn `GetCurrentHealth`
  (returns (CurrentHealth :type "Float (double-precision)"))
  (return (`self.CurrentHealth`)))

(fn `IsAlive`
  (returns (ReturnValue :type Boolean))
  (return (> (`self.CurrentHealth`) 0.0)))

(fn `OnRep_CurrentHealth`
  (`self.OnHealthChanged`))

(fn `OnTakeAnyDamage`
  (params (DamagedActor :type "Actor Object Reference") (Damage :type "Float (double-precision)") (DamageType :type "DamageType Object Reference") (InstigatedBy :type "Controller Object Reference") (DamageCauser :type "Actor Object Reference"))
  (bind _output_get (set `self.CurrentHealth` (`KismetMathLibrary.FMax` (- (`self.CurrentHealth`) Damage))))
  (if (== _output_get 0.0)
    (set `Actor.bCanBeDamaged` false (`self.GetOwner`))
    (`self.OnDeath`)))

(fn `ReceiveBeginPlay`
  (bind _returnvalue (`self.GetOwner`))
  (if (or (`KismetSystemLibrary.IsServer`) (`KismetSystemLibrary.IsStandalone`))
    (`|ExecutionSequence`
      (:`then_0`
        (`/Engine/EditorBlueprintResources/StandardMacros.IsValid` _returnvalue
          (:`Is Valid`
            (add `Actor.OnTakeAnyDamage` _returnvalue (`|CreateDelegate` :!event `OnTakeAnyDamage`))))))))
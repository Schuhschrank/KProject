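; Base-style interactable task that one BP_KCharacterChild at a time progresses by spending its progress points, and that can be sabotaged once completed.
; Interacting starts a looping one-second timer, and each iteration converts points into progress until interaction ends or points run short.
; Registers with BP_KGameMode while incomplete and unregisters on completion, toggling the Completed indicator.
; Begin play and reset logic run only on authority.
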(event `/Game/Blueprints/BI_Generic.Interact`
  (params (PlayerPawn :type "Pawn Object Reference"))
  (`/Engine/EditorBlueprintResources/StandardMacros.IsValid` (`self.InteractingWith`)
    (:`Is Not Valid`
      (bind _asbp_kcharacter_child (cast `/Game/Blueprints/Character/BP_KCharacterChild` PlayerPawn))
      (`/Engine/EditorBlueprintResources/StandardMacros.IsValid` _asbp_kcharacter_child
        (:`Is Valid`
          (set `self.InteractingWith` _asbp_kcharacter_child)
          (`self.IterateInteraction`)
          (bind _returnvalue (`KismetSystemLibrary.K2_SetTimerDelegate` (`|CreateDelegate` :!event `IterateInteraction`) 1.0 true))
          (set `self.Timer` _returnvalue))))))

(event `/Game/Blueprints/BI_Generic.StopInteracting`
  (params (PlayerPawn :type "Pawn Object Reference"))
  (`/Engine/EditorBlueprintResources/StandardMacros.IsValid` PlayerPawn
    (:`Is Valid`
      (if (== PlayerPawn (`self.InteractingWith`))
        (`self.EndInteraction`)))))

(event `PlaySound`
  (`GameplayStatics.PlaySoundAtLocation` "/Game/Audio/fart_noise_Cue.fart_noise_Cue" (`self.K2_GetActorLocation`) (struct) 1.0 1.0 0.0 null null self))

(fn `AddToProgress`
  (params (Amount :type "Float (double-precision)"))
  (locals (bWasCompleted :type Boolean :default false))
  (set `local.bWasCompleted` (>= (`self.Progress`) 1.0))
  (bind _output_get (set `self.Progress` (+ Amount (`self.Progress`))))
  (`self.PlaySound`)
  (if (and (>= _output_get 1.0) (not (`local.bWasCompleted`)))
    (`self.Unregister`)))

(fn `EndInteraction`
  (`KismetSystemLibrary.K2_ClearAndInvalidateTimerHandle` (`self.Timer`))
  (set `self.InteractingWith` null))

(fn `IterateInteraction`
  (bind _returnvalue (`self.GetRateOfProgress`))
  (bind _interactingwith (`self.InteractingWith`))
  (bind _progresspoints (`/Game/Blueprints/Character/BP_KCharacterChild.GetProgressPoints` _interactingwith))
  (`/Engine/EditorBlueprintResources/StandardMacros.IsValid` _interactingwith
    (:`Is Valid`
      (if (>= _progresspoints _returnvalue)
        (`/Game/Blueprints/Character/BP_KCharacterChild.SetProgressPoints` (`self.InteractingWith`) (- _progresspoints _returnvalue))
        (`self.AddToProgress` (`self.GetRateOfProgress`))
        (else
          (`self.EndInteraction`))))
    (:`Is Not Valid`
      (`self.EndInteraction`))))

(fn `K2_OnReset`
  (locals (bWasCompleted :type Boolean :default false))
  (`/Engine/EditorBlueprintResources/ActorMacros.Switch Has Authority`
    (:`Authority`
      (`|ExecutionSequence`
        (:`then_0`
          (set `local.bWasCompleted` (>= (`self.Progress`) 1.0))
          (set `self.Progress` 0.0))
        (:`then_1`
          (`self.EndInteraction`))
        (:`then_2`
          (if (`local.bWasCompleted`)
            (`self.Register`)))))))

(fn `ReceiveBeginPlay`
  (`/Engine/EditorBlueprintResources/ActorMacros.Switch Has Authority`
    (:`Authority`
      (`self.Register`))))

(fn `Register`
  (`SceneComponent.SetVisibility` (`self.Completed`) false false)
  (bind _asbp_kgame_mode (cast `/Game/Blueprints/GameFramework/BP_KGameMode` (`GameplayStatics.GetGameMode`)))
  (`/Game/Blueprints/GameFramework/BP_KGameMode.RegisterTask` _asbp_kgame_mode))

(fn `Sabotage`
  (locals (bWasCompleted :type Boolean :default false))
  (if (>= (`self.Progress`) 1.0)
    (bind _output_get (set `self.Progress` (`KismetMathLibrary.FMin` (* (`self.Progress`) 0.5) 0.67)))
    (`self.Register`)
    (`self.PlaySound`)))

(fn `Unregister`
  (`SceneComponent.SetVisibility` (`self.Completed`) true false)
  (bind _asbp_kgame_mode (cast `/Game/Blueprints/GameFramework/BP_KGameMode` (`GameplayStatics.GetGameMode`)))
  (`/Game/Blueprints/GameFramework/BP_KGameMode.UnregisterTask` _asbp_kgame_mode))

(fn `UserConstructionScript`)
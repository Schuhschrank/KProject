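; BP_PPSource is an interactable source that gives progress points to the BP_KCharacterChild interacting with it.
; Interact stores the character, adds points immediately and starts a looping half-second timer for further increments.
; IterateInteraction adds GetRateOfProgress while the character is below GetMaxPP, otherwise clearing the timer.
; StopInteracting also clears the timer, as does a reset on the authority.
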(event `/Game/Blueprints/BI_Generic.Interact`
  (params (PlayerPawn :type "Pawn Object Reference"))
  (bind _asbp_kcharacter_child (cast `/Game/Blueprints/Character/BP_KCharacterChild` PlayerPawn))
  (`/Engine/EditorBlueprintResources/StandardMacros.IsValid` _asbp_kcharacter_child
    (:`Is Valid`
      (set `self.InteractingWith` _asbp_kcharacter_child)
      (`self.IterateInteraction`)
      (bind _returnvalue (`KismetSystemLibrary.K2_SetTimerDelegate` (`|CreateDelegate` :!event `IterateInteraction`) 0.5 true))
      (set `self.Timer` _returnvalue))))

(event `/Game/Blueprints/BI_Generic.StopInteracting`
  (params (PlayerPawn :type "Pawn Object Reference"))
  (`KismetSystemLibrary.K2_ClearAndInvalidateTimerHandle` (`self.Timer`)))

(fn `IterateInteraction`
  (bind _interactingwith (`self.InteractingWith`))
  (bind _progresspoints (`/Game/Blueprints/Character/BP_KCharacterChild.GetProgressPoints` _interactingwith))
  (`/Engine/EditorBlueprintResources/StandardMacros.IsValid` _interactingwith
    (:`Is Valid`
      (if (< _progresspoints (`self.GetMaxPP`))
        (`/Game/Blueprints/Character/BP_KCharacterChild.SetProgressPoints` (`self.InteractingWith`) (+ _progresspoints (`self.GetRateOfProgress`)))
        (else
          (`KismetSystemLibrary.K2_ClearAndInvalidateTimerHandle` (`self.Timer`) :!label _label))))
    (:`Is Not Valid`
      (goto _label))))

(fn `K2_OnReset`
  (locals (bWasCompleted :type Boolean :default false))
  (`/Engine/EditorBlueprintResources/ActorMacros.Switch Has Authority`
    (:`Authority`
      (`KismetSystemLibrary.K2_ClearAndInvalidateTimerHandle` (`self.Timer`)))))

(fn `UserConstructionScript`)
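; BP_TPlayerController is a test player controller that triggers game-mode restart and reset operations from debug keys.
; On BeginPlay it caches BP_TGameModeBase, and local controllers add the WB_TDebug widget with cursor input enabled.
; Keys call restart, game reset and several player reset variants on the game mode, while Z toggles between UI and game-only input.
; Tick prints whether a spectator pawn is valid.
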(event `self.ReceiveBeginPlay`
  (`|ExecutionSequence`
    (:`then_0`
      (bind _asbp_tgame_mode_base (cast `/Game/Testing/BP_TGameModeBase` (`GameplayStatics.GetGameMode`)))
      (set `self.As BP TGame Mode Base` _asbp_tgame_mode_base))
    (:`then_1`
      (if (`self.IsLocalPlayerController`)
        (bind _returnvalue (`|CreateWidget` "/Game/Testing/WB_TDebug.WB_TDebug_C" self))
        (`UserWidget.AddToViewport` _returnvalue 0)
        (`WidgetBlueprintLibrary.SetInputMode_GameAndUIEx` self null)
        (set `self.bShowMouseCursor` true)))))

(event `ResetLevel`
  (`GameModeBase.ResetLevel` (`GameplayStatics.GetGameMode`)))

(event `Key|P`
  (params (Key :type "Key Structure"))
  (:`Pressed`
    (`self.RestartPlayer`)))

(event `RestartPlayer`
  (`GameModeBase.RestartPlayer` (`GameplayStatics.GetGameMode`) self))

(event `Key|C`
  (params (Key :type "Key Structure"))
  (:`Pressed`
    (`self.ResetPlayer`)))

(event `ResetPlayer`
  (`TGameModeBase.ResetPlayer` (`self.As BP TGame Mode Base`) self))

(event `Key|G`
  (params (Key :type "Key Structure"))
  (:`Pressed`
    (`TGameModeBase.ResetGame` (`self.As BP TGame Mode Base`))))

(event `Key|One`
  (params (Key :type "Key Structure"))
  (:`Pressed`
    (`self.ResetPlayerServer`)))

(event `ResetPlayerServer`
  (`TGameModeBase.ResetPlayerServer` (`self.As BP TGame Mode Base`) self))

(event `Key|Two`
  (params (Key :type "Key Structure"))
  (:`Pressed`
    (`self.ResetPlayerClient`)))

(event `ResetPlayerClient`
  (`TGameModeBase.ResetPlayerClient` (`self.As BP TGame Mode Base`) self))

(event `Key|V`
  (params (Key :type "Key Structure"))
  (:`Pressed`
    (`self.ResetPlayerReversed`)))

(event `ResetPlayerReversed`
  (`TGameModeBase.ResetPlayerReversed` (`self.As BP TGame Mode Base`) self))

(event `Key|Z`
  (params (Key :type "Key Structure"))
  ;[1 1 1] Open and close in-game menu
  (:`Pressed`
    (`/Engine/EditorBlueprintResources/StandardMacros.FlipFlop`
      (:`A`
        (`WidgetBlueprintLibrary.SetInputMode_GameAndUIEx` self null)
        (set `self.bShowMouseCursor` true))
      (:`B`
        (`WidgetBlueprintLibrary.SetInputMode_GameOnly` self)
        (set `self.bShowMouseCursor` false)))))

(event `UnPossessServer`
  (`self.UnPossess`))

(event `self.SomePawn.OnDeath`
  (params (Player :type "Controller Object Reference")))

(fn `ReceiveTick`
  (params (DeltaSeconds :type "Float (double-precision)"))
  (`KismetSystemLibrary.PrintString` (`KismetStringLibrary.Conv_BoolToString` (`KismetSystemLibrary.IsValid` (`self.GetSpectatorPawn`))) true false (struct :`G` 0.66 :`B` 1.0 :`A` 1.0) 0.0))

(fn `UserConstructionScript`)